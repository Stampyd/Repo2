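; SimpleAI is a basic AI-controlled actor that chases the player when nearby.
; Every Tick it checks distance to the player character and uses simple move-to-actor within a fixed radius, otherwise moving to a fixed location with only Z specified.
; An ApplyDamage function subtracts damage from Health, but the zero-health check is unused, so nothing here handles death.
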(event `self.ReceiveTick`
  (params (DeltaSeconds :type "Float (single-precision)"))
  (bind _returnvalue (`self.GetController` self))
  (if (< (`self.GetDistanceTo` (`GameplayStatics.GetPlayerCharacter` 0)) 500.0)
    (`NavigationSystem.SimpleMoveToActor` _returnvalue (`GameplayStatics.GetPlayerCharacter` 0))
    (else
      (`NavigationSystem.SimpleMoveToLocation` _returnvalue (0.0 0.0 110.0)))))

(fn `apply damage`
  (params (damage :type "Float (double-precision)" :default 0.0))
  (set `self.health` (- (`self.health`) damage)))

(fn `UserConstructionScript`)